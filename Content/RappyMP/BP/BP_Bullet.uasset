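; BP_Bullet is a multiplayer projectile that damages players and self-destructs on impact or when its lifetime timer expires.
; The server moves it forward each Tick by setting its location without sweep, and handles collider overlaps.
; Overlaps with non-owner actors harm any BP_Player, multicast an impact particle effect at the bullet's location, then destroy the bullet through a server-side event.
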(event OnComponentBeginOverlap(Collider)
  (params (OverlappedComponent :type Primitive%20Component%20Object%20Reference) (OtherActor :type Actor%20Object%20Reference) (OtherComp :type Primitive%20Component%20Object%20Reference) (OtherBodyIndex :type Integer) (bFromSweep :type Boolean) (SweepResult :type Hit%20Result%20Structure%20%28by%20ref%29))
  (if (Networking|IsServer)
    (Development|PrintString (Utilities|GetDisplayName OtherComp))
    (CallFunction|CollisionResponseServerSide OtherActor (Transformation|GetActorLocation))))

(event Custom|SelfDestruct
  ;[1 1 1] Lifecycle
  (CallFunction|SelfDestructServerSide))

(event Custom|SelfDestruct_ServerSide
  ;[1 1 1] Lifecycle
  (Actor|DestroyActor))

(event Custom|Move_ServerSide
  ;[1 1 1] Movement
  (Transformation|SetActorLocation (+ (Transformation|GetActorLocation) (* (Transformation|GetActorForwardVector) (* (stale EventTick DeltaSeconds) (Variables|Default|GetBulletVelocity)))) false false))

(event Custom|CollisionResponse_ServerSide
  (params (HitActor :type Actor%20Object%20Reference) (HitLocation :type Vector))
  (if (!= HitActor (Components|GetOwner))
    (bind _asbp_player (Utilities|Casting|CastToBP_Player HitActor)
      (:then
        (Default|Harm _asbp_player (Variables|Default|GetDamage)))
      (:CastFailed
        _))
    (CallFunction|MulticastHitEvent HitLocation)
    (CallFunction|SelfDestructServerSide)))

(event Custom|SpawnHitEffect
  (params (SpawnLocation :type Vector))
  (Effects|SpawnEmitteratLocation "/Game/RappyMP/Effects/P_Impact.P_Impact" SpawnLocation "0, 0, 0" "1.000000,1.000000,1.000000" true "AutoRelease"))

(event Custom|Multicast_HitEvent
  (params (SpawnLocation :type Vector))
  (CallFunction|SpawnHitEffect SpawnLocation))

(event EventBeginPlay
  ;[1 1 1] Lifecycle
  (Utilities|Time|SetTimerbyEvent (delegate Custom|SelfDestruct) (Variables|Default|GetLifetime)))

(event Collision|EventActorBeginOverlap
  (params (OtherActor :type Actor%20Object%20Reference)))

(event EventTick
  (params (DeltaSeconds :type Float%20%28single-precision%29))
  (if (Networking|IsServer)
    (CallFunction|MoveServerSide)))

(fn ConstructionScript)