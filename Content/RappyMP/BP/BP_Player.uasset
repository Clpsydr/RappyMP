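; BP_Player is the multiplayer player pawn that handles firing, damage and team identity.
; Server-side firing spawns a projectile at FireOrigin, then a fire-rate timer restores ReadyToFire, which is also pushed client-side to the visual status indicator every tick.
; BPPlayerStats holds HP and fire rate, with damage subtracted through a server event.
; Team changes pass from server to multicast, tinting mesh materials by TeamID, initially taken from the player controller.
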(event Custom|Fire_Serverside
  (bind _self self)
  (bind _fireorigin (Variables|Default|GetFireOrigin))
  (bind _returnvalue (Transformation|GetWorldTransform _fireorigin))
  ;[1 1 1] Firing
  (if (Variables|Default|GetReadyToFire)
    (Game|SpawnActorfromClass (Variables|Default|GetProjType) (Math|Transform|MakeTransform (+ (.location _returnvalue) "0, 0, 0") (.rotation _returnvalue)) "AlwaysSpawn" _self _self)
    (Variables|Default|SetReadyToFire false)
    (Utilities|Time|SetTimerbyEvent (delegate Custom|ReloadDone) (Variables|/Game/RappyMP/BP/BP_PlayerStats.BP_PlayerStats_C|GetFirerate (Variables|Default|GetBP_PlayerStats)))))

(event Custom|SetTeamSkin
  ;[1 1 1] Dynamic mat setup to represent team
  (Rendering|Material|SetVectorParameterValueonMaterials (Variables|Character|GetMesh) "TeamColor" (Utilities|Select :Index (Variables|Default|GetTeamID) :Option%200 (Math|Vector|MakeVector 0.5 0.5 0.5) :Option%201 (Math|Vector|MakeVector 1.0 0.0 0.0) :Option%202 (Math|Vector|MakeVector 0.0 0.0 1.0))))

(event Custom|ReloadUpdate_ClientSide
  (params (ReloadState :type Boolean))
  ;[1 1 1] Clientside reload manage
  (bind _output_get (Variables|Default|SetReadyToFire ReloadState))
  (Default|UpdateFireIndice (Variables|Default|GetBP_PlayerVisualStatus) _output_get))

(event Custom|Harm
  (params (Damage%20Value :type Float%20%28single-precision%29))
  ;[1 1 1] HP/stats change
  (CallFunction|HarmServerSide Damage%20Value))

(event Custom|ReloadDone
  ;[1 1 1] notifier and reload state done
  (bind _output_get (Variables|Default|SetReadyToFire true))
  (CallFunction|ReloadUpdateClientSide _output_get))

(event Custom|Harm_ServerSide
  (params (DamageValue :type Float%20%28single-precision%29))
  (bind _bp_playerstats (Variables|Default|GetBP_PlayerStats))
  ;[1 1 1] HP/stats change
  (Variables|/Game/RappyMP/BP/BP_PlayerStats.BP_PlayerStats_C|SetHPCurrent _bp_playerstats (- (Variables|/Game/RappyMP/BP/BP_PlayerStats.BP_PlayerStats_C|GetHPCurrent _bp_playerstats) DamageValue)))

(event Custom|UpdateName
  (bind _asbp_player_controller (Utilities|Casting|CastToBP_PlayerController (Pawn|GetController)))
  (Default|UpdateName (Variables|Default|GetBP_PlayerVisualStatus) (Variables|/Game/RappyMP/BP/BP_PlayerController.BP_PlayerController_C|GetPlayerName _asbp_player_controller)))

(event Custom|ChangedTeam_ServerSide
  ;[1 1 1] Team id and skin setup
  (CallFunction|ChangedTeamMultiCast))

(event Custom|ChangedTeam_MultiCast
  ;[1 1 1] Team id and skin setup
  (CallFunction|SetTeamSkin))

(event Custom|AssignToNewTeam_ServerSide
  (params (NewID :type Byte))
  ;[1 1 1] Team id and skin setup
  (Variables|Default|SetTeamID NewID)
  (CallFunction|ChangedTeamMultiCast))

(event EventBeginPlay
  (bind _bp_playerstats (Variables|Default|GetBP_PlayerStats))
  (Default|InitHPServerSide _bp_playerstats)
  ;[1 1 1] BeginPlay
  (Utilities|Time|SetTimerbyEvent (delegate Custom|ReloadDone) (Variables|/Game/RappyMP/BP/BP_PlayerStats.BP_PlayerStats_C|GetFirerate _bp_playerstats))
  (bind _asbp_player_controller (Utilities|Casting|CastToBP_PlayerController (Pawn|GetController))
    (:then
      (CallFunction|AssigntoNewTeamServerSide (Variables|/Game/RappyMP/BP/BP_PlayerController.BP_PlayerController_C|GetTeamID _asbp_player_controller)))
    (:CastFailed
      (CallFunction|SetTeamSkin))))

(event Collision|EventActorBeginOverlap
  (params (OtherActor :type Actor%20Object%20Reference)))

(event EventTick
  (params (DeltaSeconds :type Float%20%28single-precision%29))
  ;[1 1 1] DT update
  (CallFunction|ReloadUpdateClientSide (Variables|Default|GetReadyToFire)))

(fn ConstructionScript)

(fn OnRepReadytoFire)

(fn GetCtrlTeamID
  (bind _asbp_player_controller (Utilities|Casting|CastToBP_PlayerController (Pawn|GetController))
    (:then
      (return (Variables|/Game/RappyMP/BP/BP_PlayerController.BP_PlayerController_C|GetTeamID _asbp_player_controller)))
    (:CastFailed
      (return 0))))