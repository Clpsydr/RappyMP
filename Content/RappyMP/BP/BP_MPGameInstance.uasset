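; Game Instance for RappyMP that manages LAN multiplayer sessions: hosting, browsing and joining games.
; Hosting creates a session and opens the Arena level as a listen server.
; Searches store results and feed server stats with session references to ServerListUI; joining takes either a chosen session or a single search result.
; Session failures and network or travel errors are printed on screen.
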(event Custom|CreateNewGame
  ;[1 1 1] Create game
  (|Session (Game|GetPlayerController 0) 16 true
    (:OnSuccess
      (Game|OpenLevel(byName) "Arena" true "listen"))
    (:OnFailure
      (Development|PrintString "Unable to open session"))))

(event Custom|FindGames
  ;[1 1 1] save and display the game list
  (bind _results (|FindSessions (Game|GetPlayerController 0) 10 true)
    (:OnSuccess
      (bind _output_get (Variables|Default|SetSessionList _results))
      (for _array_element _output_get
        (Default|AddNewEntry (Variables|Default|GetServerListUI) (Utilities|Struct|MakeServerStats (Class|FindSessionsCallbackProxy|GetServerName _array_element) (Math|Conversions|ToFloat(Integer) (Class|FindSessionsCallbackProxy|GetPinginMs _array_element)) (Class|FindSessionsCallbackProxy|GetCurrentPlayers _array_element) (Class|FindSessionsCallbackProxy|GetMaxPlayers _array_element) _array_element))))
    (:OnFailure
      (Development|PrintString "Error: Can't find sessions"))))

(event Custom|JoinGame
  (bind _returnvalue (Game|GetPlayerController 0))
  ;[1 1 1] Join logic
  (bind _results (|FindSessions _returnvalue 1 true)
    (:OnSuccess
      (for _array_element _results
        (|JoinSession _returnvalue _array_element
          (:OnFailure
            (Development|PrintString "Error: Cannot join session")))))
    (:OnFailure
      (Development|PrintString "Error: Can't find sessions"))))

(event Custom|JoinSpecificGame
  (params (TargetedSession :type Blueprint%20Session%20Result%20Structure))
  ;[1 1 1] Join logic
  (|JoinSession (Game|GetPlayerController 0) TargetedSession
    (:OnFailure
      (Development|PrintString "Error: Cannot join session"))))

(event EventHandleNetworkError
  (params (FailureType :type ENetworkFailure%20Enum :default "NetDriverAlreadyExists") (bIsServer :type Boolean))
  ;[1 1 1] Errors
  (Development|PrintString (Utilities|String|Append "Network error: " (Utilities|String|EnumtoString FailureType) (Utilities|String|SelectString "on server" "on client" bIsServer)) true true "(R=1.000000,G=0.020644,B=0.000000,A=1.000000)" 1e+01))

(event EventHandleTravelError
  (params (FailureType :type ETravelFailure%20Enum :default "NoLevel"))
  ;[1 1 1] Errors
  (Development|PrintString (Utilities|String|Append "Travel error: " (Utilities|String|EnumtoString FailureType)) true true "(R=1.000000,G=0.016751,B=0.000000,A=1.000000)" 1e+01))

(fn AddNewServerInfo
  (params (NewStats :type Server%20Stats%20Structure))
  (Utilities|Array|Add (Variables|Default|GetServerList) NewStats)
  (Default|AddNewEntry (Variables|Default|GetServerListUI) NewStats))