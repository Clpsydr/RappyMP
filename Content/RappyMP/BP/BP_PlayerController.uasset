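; Player controller for a team-based multiplayer mode that drives BP_Player with look, camera-relative movement, jump and held-trigger fire.
; On BeginPlay it caches the pawn via GetPlayerPawn(0), requests team 0 and updates its name.
; Holding Fire calls the pawn's server-side fire every Tick, with no rate limit here.
; Game-mode-launched team assignment stores TeamID and builds a random bird-themed player name; key 2 calls BP_DMMode's team stats.
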(event Custom|SetTeamID
  (params (NewID :type Byte))
  ;[1 1 1] Param assign - launched from gamemode
  (CallFunction|SetTeamIDServerSide NewID))

(event Custom|SetTeamID_ServerSide
  (params (NewID :type Byte))
  ;[1 1 1] Param assign - launched from gamemode
  (bind _output_get (Variables|Default|SetTeamID NewID))
  (Variables|Default|SetPlayerName (Utilities|String|Append "Team" (Utilities|String|ToString(Byte) _output_get) "_" (Utilities|Select :Index (Math|Random|RandomInteger 4) :Option%200 (Utilities|String|MakeLiteralString "Birb") :Option%201 (Utilities|String|MakeLiteralString "Burd") :Option%202 (Utilities|String|MakeLiteralString "Borb") :Option%203 (Utilities|String|MakeLiteralString "Briby")))))

(event EventBeginPlay
  ;[1 1 1] player pawn init
  (bind _asbp_player (Utilities|Casting|CastToBP_Player (Game|Player|GetPlayerPawn 0))
    (:then
      (bind _output_get (Variables|Default|SetPlayerPawn _asbp_player))
      (Default|AssigntoNewTeamServerSide _output_get)
      (Default|UpdateName _output_get))
    (:CastFailed
      (Development|PrintString "Failed to obtain controlled pawn"))))

(event EventTick
  (params (DeltaSeconds :type Float%20%28single-precision%29))
  (if (Variables|Default|GetRapidFire)
    (Default|FireServerside (Variables|Default|GetPlayerPawn))))

(event Input|ActionEvents|InputActionJump
  (params (Key :type Key%20Structure :default "None"))
  (bind _playerpawn (Variables|Default|GetPlayerPawn))
  ;[1 1 1] Movement Controls
  (:Pressed
    (Character|Jump _playerpawn))
  (:Released
    (Character|StopJumping _playerpawn)))

(event Input|ActionEvents|InputActionFire
  (params (Key :type Key%20Structure :default "None"))
  (:Pressed
    (Variables|Default|SetRapidFire true))
  (:Released
    (Variables|Default|SetRapidFire false)))

(event Input|AxisEvents|InputAxisTurn
  (params (AxisValue :type Float%20%28single-precision%29))
  ;[1 1 1] Camera Controls
  (Class|PlayerController|AddYawInput AxisValue))

(event Input|AxisEvents|InputAxisLookUp
  (params (AxisValue :type Float%20%28single-precision%29))
  ;[1 1 1] Camera Controls
  (Class|PlayerController|AddPitchInput AxisValue))

(event Input|AxisEvents|InputAxisMoveForward
  (params (AxisValue :type Float%20%28single-precision%29))
  (bind _playerpawn (Variables|Default|GetPlayerPawn))
  ;[1 1 1] Movement Controls
  (if (Utilities|IsValid _playerpawn)
    (Pawn|Input|AddMovementInput _playerpawn (Math|Vector|GetForwardVector (Math|Rotator|MakeRotator 0.0 0.0 (.Yaw (Math|Rotator|BreakRotator (Pawn|GetControlRotation :!class /Script/Engine.Controller))))) AxisValue false)))

(event Input|AxisEvents|InputAxisMoveRight
  (params (AxisValue :type Float%20%28single-precision%29))
  (bind _playerpawn (Variables|Default|GetPlayerPawn))
  ;[1 1 1] Movement Controls
  (if (Utilities|IsValid _playerpawn)
    (Pawn|Input|AddMovementInput _playerpawn (Math|Vector|GetRightVector (Math|Rotator|MakeRotator 0.0 0.0 (.Yaw (Math|Rotator|BreakRotator (Pawn|GetControlRotation :!class /Script/Engine.Controller))))) AxisValue false)))

(event Input|KeyboardEvents|2
  (params (Key :type Key%20Structure :default "None"))
  ;[1 1 1] Checking out team compo
  (:Pressed
    (bind _asbp_dmmode (Utilities|Casting|CastToBP_DMMode (Game|GetGameMode)))
    (Default|ServerStats _asbp_dmmode)))

(fn ConstructionScript)