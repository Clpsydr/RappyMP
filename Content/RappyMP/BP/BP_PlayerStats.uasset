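; BP_PlayerStats is a component holding a player's replicated stats: max and current HP, fire rate and reloading state.
; A server-side init fills current HP to max, and only the current HP RepNotify reacts, refreshing visuals and printing HP for debugging.
; The refresh sends the HP ratio to the owner's BP_PlayerVisualStatus component, printing a notice if that component is not valid yet.
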(event Custom|UpdateVisuals
  (CallFunction|UpdateWidget))

(event Custom|InitHP_ServerSide
  (Variables|Default|SetHPCurrent (Variables|Default|GetHPMax)))

(event EventBeginPlay)

(event EventTick
  (params (DeltaSeconds :type Float%20%28single-precision%29)))

(fn OnRepHPMax)

(fn OnRepHPCurrent
  (CallFunction|UpdateVisuals)
  (Development|PrintString (Utilities|String|Append (Utilities|String|ToString(Float) (Variables|Default|GetHPCurrent)) " / " (Utilities|String|ToString(Float) (Variables|Default|GetHPMax))) true true "(R=1.000000,G=0.000000,B=0.028639,A=1.000000)"))

(fn OnRepFirerate)

(fn OnRepReloading)

(fn GetHPRatio
  (return (Math|Float|SafeDivide (Variables|Default|GetHPCurrent) (Variables|Default|GetHPMax))))

(fn UpdateWidget
  (bind _returnvalue (Components|GetOwner))
  (bind _returnvalue_2 (Actor|GetComponentbyClass _returnvalue "/Game/RappyMP/UI/BP_PlayerVisualStatus.BP_PlayerVisualStatus_C"))
  (if (Utilities|IsValid _returnvalue_2)
    (bind _hpratio (CallFunction|GetHPRatio))
    (Default|UpdatePlayerWidgetServerSide _returnvalue_2 _hpratio)
    (else
      (Development|PrintString "HP widget not ready yet"))))