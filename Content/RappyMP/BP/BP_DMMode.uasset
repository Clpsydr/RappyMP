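; BP_DMMode is a game mode, apparently for deathmatch, that splits joining players into two teams.
; On post-login it adds the BP_PlayerController to the smaller team array, with ties going to Team 2, and sets the controller's TeamID.
; On logout it uses that TeamID to find and remove the player from the team.
; A ServerStats event prints both rosters, and logins and logouts print debug messages.
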(event Custom|ServerStats
  ;[1 1 1] Prints out report on team composition (spoiler: they're both empty)
  (Development|PrintString "Team1: ")
  (for _array_element (Variables|Default|GetTeam1)
    (Development|PrintString (Utilities|String|Append (Variables|/Game/RappyMP/BP/BP_PlayerController.BP_PlayerController_C|GetPlayerName _array_element) ", ")))
  (Development|PrintString "Team2: ")
  (for _array_element_2 (Variables|Default|GetTeam2)
    (Development|PrintString (Utilities|String|Append (Variables|/Game/RappyMP/BP/BP_PlayerController.BP_PlayerController_C|GetPlayerName _array_element_2) ", "))))

(event EventTick
  (params (DeltaSeconds :type Float%20%28single-precision%29)))

(event EventPostLogin
  (params (NewPlayer :type Player%20Controller%20Object%20Reference))
  ;[1 1 1] Login, assigning player to smaller team
  (bind _asbp_player_controller (Utilities|Casting|CastToBP_PlayerController NewPlayer)
    (:then
      (bind (_smallerteamid _smallerteam) (CallFunction|GetLesserTeam))
      (Default|SetTeamID _asbp_player_controller _smallerteamid)
      (Utilities|Array|Add _smallerteam _asbp_player_controller)
      (Development|PrintString (Utilities|String|Append "Team " (Utilities|String|ToString(Byte) _smallerteamid) " gets unit, total " (Utilities|String|ToString(Integer) (Utilities|Array|Length _smallerteam)) " players")))
    (:CastFailed
      (Development|PrintString "Error on postlogin: wrong player controller"))))

(event EventOnLogout
  (params (ExitingController :type Controller%20Object%20Reference))
  ;[1 1 1] Lgout, kicking player from the team
  (bind _asbp_player_controller (Utilities|Casting|CastToBP_PlayerController ExitingController))
  (bind _playerteam (CallFunction|FindinATeam (Variables|/Game/RappyMP/BP/BP_PlayerController.BP_PlayerController_C|GetTeamID _asbp_player_controller)))
  (bind _returnvalue (Utilities|Array|RemoveItem _playerteam _asbp_player_controller))
  (if _returnvalue
    (Development|PrintString "Player has quit, but you need to update more than that?")
    (else
      (Development|PrintString "on logout, cant find player in team"))))

(fn ConstructionScript)

(fn GetLesserTeam
  (bind _team1 (Variables|Default|GetTeam1))
  (bind _team2 (Variables|Default|GetTeam2))
  (if (< (Utilities|Array|Length _team1) (Utilities|Array|Length _team2))
    (return 1 _team1)
    (else
      (return 2 _team2))))

(fn FindinATeam
  (params (PlayerTeamID :type Byte))
  (return (Utilities|Select :Index (- PlayerTeamID 1) :Option%200 (Variables|Default|GetTeam1) :Option%201 (Variables|Default|GetTeam2))))